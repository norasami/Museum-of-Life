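; Spline-driven chain builder whose construction script lays copies of an input link mesh along a spline.
; Link spacing comes from mesh bounds, offset and size; RotateEvens alternates a 90-degree roll, otherwise every link gets it.
; Each link is its own InstancedStaticMesh component with a dynamic material: plastic striped in two colors by counter and DoN, or metal with rust, roughness, tiling and tint parameters.
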(fn ConstructionScript
  (bind _size (Variables|ChainSettings|GetSize))
  (bind _colorored_units (Variables|PlasticMaterial|GetColorored%20Units))
  (bind _spline (Variables|Default|GetSpline))
  ;[1 1 1] Local Variable that determine the spacing of the meshes
  (Variables|Default|SetSpacing (* (+ (.x (.boxextent (StaticMesh|GetBounds (Variables|ChainSettings|GetInput%20Mesh)))) (Variables|ChainSettings|GetChain%20Offset)) (Variables|ChainSettings|GetSize)))
  ;[1 1 1] Get spline length and calculates the number of chain links
  (for _index (range 0 (.ReturnValue (Math|Float|Division(WholeandRemainder) (Spline|GetSplineLength (Variables|Default|GetSpline)) (Variables|Default|GetSpacing))))
    ;[1 1 1] Positions each chain link at the spline and defines the mesh and his size
    (bind _output_get (Variables|Default|Seti-Link _index))
    (if (Variables|ChainSettings|GetRotateEvens?)
      ;;[0.9949 1 0.6783] Rotate every other link 90 degrees
      (if (> (Math|Integer|%(Integer) (Variables|Default|Geti-Link) 2) 0)
        (bind _returnvalue (AddComponent|AddInstancedStaticMeshComponent false (Math|Transform|MakeTransform (Spline|GetLocationatDistanceAlongSpline _spline (* _output_get (Variables|Default|GetSpacing)) "Local") (Math|Rotator|MakeRotator (+ (.Roll (Math|Rotator|BreakRotator (Spline|GetRotationatDistanceAlongSpline _spline (* _output_get (Variables|Default|GetSpacing)) "Local"))) 9e+01) (.Pitch (Math|Rotator|BreakRotator (Spline|GetRotationatDistanceAlongSpline _spline (* _output_get (Variables|Default|GetSpacing)) "Local"))) (.Yaw (Math|Rotator|BreakRotator (Spline|GetRotationatDistanceAlongSpline _spline (* _output_get (Variables|Default|GetSpacing)) "Local"))))) :!label _label))
        (Variables|Default|SetActualNode _returnvalue)
        (else
          (bind _returnvalue_2 (AddComponent|AddInstancedStaticMeshComponent false (Math|Transform|MakeTransform (Spline|GetLocationatDistanceAlongSpline _spline (* _output_get (Variables|Default|GetSpacing)) "Local") (Spline|GetRotationatDistanceAlongSpline _spline (* _output_get (Variables|Default|GetSpacing)) "Local"))))
          (Variables|Default|SetActualNode _returnvalue_2)))
      (else
        (goto _label)))
    (Components|StaticMesh|SetStaticMesh (Variables|Default|GetActualNode) (Variables|ChainSettings|GetInput%20Mesh))
    (Transformation|SetWorldScale3D (Variables|Default|GetActualNode) (Math|Vector|MakeVector _size _size _size))
    ;[1 1 1] Test for the chain material
    (if (Variables|ChainSettings|GetPlastic?)
      ;[1 1 1] Set "Plastic" dynamic material instance
      (bind _returnvalue_3 (Rendering|Material|CreateDynamicMaterialInstance (Variables|Default|GetActualNode) 0 (Variables|PlasticMaterial|GetPlastic%20Material) "None" :!class /Script/Engine.PrimitiveComponent))
      (Variables|Default|SetActualMaterial _returnvalue_3)
      ;[1 1 1] Paint the chain links with "Color 01" value. If the count passes the value of "Colored Units" the link is painted with "Color 02" value
      (bind _result (Math|Integer|IncrementInt (Variables|Default|GetStripeN))
        (:%20%20
          (if (> _result (Variables|PlasticMaterial|GetColorored%20Units))
            (bind _counter (Utilities|FlowControl|DoN _colorored_units :!label _label_2)
              (:Exit
                (Rendering|Material|SetVectorParameterValue (Variables|Default|GetActualMaterial) "Color" (Variables|PlasticMaterial|GetColor%2002) :!class /Script/Engine.MaterialInstanceDynamic)
                (if (>= _counter _colorored_units)
                  (Utilities|FlowControl|Sequence
                    (:then_0
                      (Variables|Default|SetStripeN 0))
                    (:then_1
                      (goto _label_2 Reset))))))
            (else
              (Rendering|Material|SetVectorParameterValue (Variables|Default|GetActualMaterial) "Color" (Variables|PlasticMaterial|GetColor%2001) :!class /Script/Engine.MaterialInstanceDynamic)))))
      (else
        ;[1 1 1] Set "Metal" dynamic material instance
        (bind _returnvalue_4 (Rendering|Material|CreateDynamicMaterialInstance (Variables|Default|GetActualNode) 0 (Variables|MetalMaterial|GetMetal%20Material) "None" :!class /Script/Engine.PrimitiveComponent))
        (bind _output_get_2 (Variables|Default|SetActualMaterial _returnvalue_4))
        ;[1 1 1] Set all values parameters on the "Metal" material
        (Rendering|Material|SetScalarParameterValue _output_get_2 "Rusty" (Variables|MetalMaterial|GetRust%20Ammount) :!class /Script/Engine.MaterialInstanceDynamic)
        (Rendering|Material|SetScalarParameterValue (Variables|Default|GetActualMaterial) "Roughness" (Variables|MetalMaterial|GetRoughness) :!class /Script/Engine.MaterialInstanceDynamic)
        (Rendering|Material|SetScalarParameterValue (Variables|Default|GetActualMaterial) "Tile UV" (Variables|MetalMaterial|GetTexture%20Tile) :!class /Script/Engine.MaterialInstanceDynamic)
        (Rendering|Material|SetVectorParameterValue (Variables|Default|GetActualMaterial) "Albedo Color" (Variables|MetalMaterial|GetMetal%20Color) :!class /Script/Engine.MaterialInstanceDynamic)
        (Rendering|Material|SetVectorParameterValue (Variables|Default|GetActualMaterial) "Rust Color" (Variables|MetalMaterial|GetRust%20Color) :!class /Script/Engine.MaterialInstanceDynamic)))))